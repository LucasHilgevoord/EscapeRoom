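; Player_Controller01 is a player pawn Blueprint, despite its controller name, that handles basic WASD movement and mouselook.
; ForwardBackward and LeftRight axes drive AddMovementInput along forward and right vectors built from control yaw alone, so camera pitch does not affect movement direction.
; Rotate and UpDown axes feed controller yaw and pitch input directly, and the construction script is empty.
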(event `InputAxis|ForwardBackward`
  (params (AxisValue :type "Float (single-precision)"))
  ;[1 1 1] WASD Player Movement
  (`self.AddMovementInput` (`KismetMathLibrary.GetForwardVector` (`KismetMathLibrary.MakeRotator` 0.0 0.0 (.yaw (`self.GetControlRotation`)))) AxisValue))

(event `InputAxis|LeftRight`
  (params (AxisValue :type "Float (single-precision)"))
  ;[1 1 1] WASD Player Movement
  (`self.AddMovementInput` (`KismetMathLibrary.GetRightVector` (`KismetMathLibrary.MakeRotator` 0.0 0.0 (.yaw (`self.GetControlRotation`)))) AxisValue))

(event `InputAxis|Rotate`
  (params (AxisValue :type "Float (single-precision)"))
  ;[1 1 1] Mouselook for player
  (`self.AddControllerYawInput` AxisValue))

(event `InputAxis|UpDown`
  (params (AxisValue :type "Float (single-precision)"))
  ;[1 1 1] Mouselook for player
  (`self.AddControllerPitchInput` AxisValue))

(fn `UserConstructionScript`)