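; Vault display actor that holds the four numbers of what appears to be a vault combination, adjusted from the VR motion controller pawn.
; Addnumber and Removenumber cast to MotionControllerPawn, then read InputNumber from the first actor found by GetAllActorsOfClass.
; That index selects which of the four counters goes up or down by one, with no clamping or wraparound.
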(fn `addnumber`
  (bind _asmotion_controller_pawn (castclass `/Game/VirtualRealityBP/Blueprints/MotionControllerPawn` "/Game/VirtualRealityBP/Blueprints/MotionControllerPawn.MotionControllerPawn_C"))
  (bind _outactors (`GameplayStatics.GetAllActorsOfClass` _asmotion_controller_pawn))
  (switch `int` (`/Game/VirtualRealityBP/Blueprints/MotionControllerPawn.input_number` (`|GetArrayItem` _outactors))
    (:`0`
      (set `self.Number_1_Numb` (+ (`self.Number_1_Numb`) 1)))
    (:`1`
      (set `self.Number_2_Numb` (+ (`self.Number_2_Numb`) 1)))
    (:`2`
      (set `self.Number_3_Numb` (+ (`self.Number_3_Numb`) 1)))
    (:`3`
      (set `self.Number_4_Numb` (+ (`self.Number_4_Numb`) 1)))))

(fn `removenumber`
  (bind _asmotion_controller_pawn (castclass `/Game/VirtualRealityBP/Blueprints/MotionControllerPawn` "/Game/VirtualRealityBP/Blueprints/MotionControllerPawn.MotionControllerPawn_C"))
  (bind _outactors (`GameplayStatics.GetAllActorsOfClass` _asmotion_controller_pawn))
  (switch `int` (`/Game/VirtualRealityBP/Blueprints/MotionControllerPawn.input_number` (`|GetArrayItem` _outactors))
    (:`0`
      (set `self.Number_1_Numb` (- (`self.Number_1_Numb`) 1)))
    (:`1`
      (set `self.Number_2_Numb` (- (`self.Number_2_Numb`) 1)))
    (:`2`
      (set `self.Number_3_Numb` (- (`self.Number_3_Numb`) 1)))
    (:`3`
      (set `self.Number_4_Numb` (- (`self.Number_4_Numb`) 1)))))

(fn `UserConstructionScript`)