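; Left locker door Blueprint that toggles its static mesh between attached and physics-simulated states.
; One custom event disables physics and attaches the supplied component to the mesh, keeping world transforms without welding.
; The other re-enables physics and detaches the actor in world space.
; Tick checks a Locked flag but does nothing with it, and the construction script is empty.
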(event `self.ReceiveTick`
  (params (DeltaSeconds :type "Float (single-precision)"))
  (if (`self.Locked`)
    _))

(event `CustomEvent_1`
  (params (AttachTo :type "SceneComponent Object Reference"))
  (`PrimitiveComponent.SetSimulatePhysics` (`self.StaticMesh`) false)
  (`SceneComponent.K2_AttachToComponent` AttachTo (`self.StaticMesh`) "None" "KeepWorld" "KeepWorld" "KeepWorld" false))

(event `CustomEvent_2`
  (`PrimitiveComponent.SetSimulatePhysics` (`self.StaticMesh`) true)
  (`self.K2_DetachFromActor` "KeepWorld" "KeepWorld" "KeepWorld"))

(fn `UserConstructionScript`)